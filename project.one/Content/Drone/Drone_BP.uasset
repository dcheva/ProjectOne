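; Player-controllable flying drone pawn that temporarily takes over possession from the player's pawn.
; Active stores the calling pawn and its controller, then possesses the drone; Deactive, bound to the Active Drone input, restores possession and destroys the drone.
; An Idle/Posses state enum gates both transitions.
; Axis inputs drive FloatingPawnMovement along actor axes and mouse look, while BeginPlay adds the drone HUD.
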(event `self.ReceiveBeginPlay`
  (bind _returnvalue (`|CreateWidget` "/Game/Drone/Drone_HUD.Drone_HUD_C"))
  (`UserWidget.AddToPlayerScreen` _returnvalue 0))

(event `InputAction|Active Drone`
  (params (Key :type "Key Structure"))
  (:`Pressed`
    (`self.Deactive`)))

(event `InputAxisKey|MouseX`
  (params (AxisValue :type "Float (single-precision)"))
  ;[1 1 1] View
  (`self.AddControllerYawInput` AxisValue))

(event `InputAxisKey|MouseY`
  (params (AxisValue :type "Float (single-precision)"))
  ;[1 1 1] View
  (`self.AddControllerPitchInput` (* AxisValue -1.0)))

(event `InputAxis|Move Up`
  (params (AxisValue :type "Float (single-precision)"))
  ;[1 1 1] Movement
  (`PawnMovementComponent.AddInputVector` (`self.FloatingPawnMovement`) (* AxisValue (`self.GetActorUpVector`)) false))

(event `InputAxis|Move Right`
  (params (AxisValue :type "Float (single-precision)"))
  ;[1 1 1] Movement
  (`PawnMovementComponent.AddInputVector` (`self.FloatingPawnMovement`) (* AxisValue (`self.GetActorRightVector`)) false))

(event `InputAxis|Move Forward`
  (params (AxisValue :type "Float (single-precision)"))
  ;[1 1 1] Movement
  (`PawnMovementComponent.AddInputVector` (`self.FloatingPawnMovement`) (* AxisValue (`self.GetActorForwardVector`)) false))

(fn `Active`
  (params (PlayerPawn :type "Character Object Reference"))
  (switch `/Game/Drone/EDrone_States` (`self.EDrone States`)
    (:`NewEnumerator0`
      (bind _output_get (set `self.Player Pawn` PlayerPawn))
      (bind _asplayer_controller (cast `PlayerController` (`self.GetController` _output_get)))
      (set `self.As Player Controller` _asplayer_controller)
      (`Controller.Possess` (`self.As Player Controller`) self)
      (set `self.EDrone States` "NewEnumerator1"))))

(fn `Deactive`
  (bind _returnvalue (`self.GetController`))
  (switch `/Game/Drone/EDrone_States` (`self.EDrone States`)
    (:`NewEnumerator1`
      (`/Engine/EditorBlueprintResources/StandardMacros.IsValid` _returnvalue
        (:`Is Valid`
          (`Controller.Possess` _returnvalue (`self.Player Pawn`))
          (`self.K2_DestroyActor`))))))

(fn `UserConstructionScript`)